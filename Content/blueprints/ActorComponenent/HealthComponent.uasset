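; Actor component that tracks the health of its owning actor, starting at the maximum on BeginPlay.
; It binds to the owner's point and radial damage events, subtracts any positive damage and clamps Health between zero and MaxHealth.
; Each damage type then fires its own dispatcher with the new Health and hit details, passing the component itself as the damaged object.
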(event EventBeginPlay
  (Variables|Default|SetHealth (Variables|Default|GetMaxHealth))
  (EventDispatchers|BindEventtoOnTakePointDamage (Components|GetOwner) (EventDispatchers|CreateEvent :!event TakePointDamage))
  (EventDispatchers|BindEventtoOnTakeRadialDamage (Components|GetOwner) (EventDispatchers|CreateEvent :!event TakeRadialDamage)))

(event EventTick
  (params (DeltaSeconds :type Float%20%28single-precision%29)))

(fn TakePointDamage
  (params (DamagedActor :type Actor%20Object%20Reference) (Damage :type Float%20%28single-precision%29) (InstigatedBy :type Controller%20Object%20Reference) (HitLocation :type Vector) (FHitComponent :type Primitive%20Component%20Object%20Reference) (BoneName :type Name) (ShotFromDirection :type Vector) (DamageType :type Damage%20Type%20Object%20Reference) (DamageCauser :type Actor%20Object%20Reference))
  (if (not (<= Damage 0.0))
    (bind _output_get (Variables|Default|SetHealth (Math|Float|Clamp(Float) (- (Variables|Default|GetHealth) Damage) 0.0 (Variables|Default|GetMaxHealth))))
    (Default|CallHandleTakePointDamge self _output_get 0.0 DamageType DamageCauser)))

(fn TakeRadialDamage
  (params (DamagedActor :type Actor%20Object%20Reference) (Damage :type Float%20%28single-precision%29) (DamageType :type Damage%20Type%20Object%20Reference) (Origin :type Vector) (HitInfo :type Hit%20Result%20Structure%20%28by%20ref%29) (InstigatedBy :type Controller%20Object%20Reference) (DamageCauser :type Actor%20Object%20Reference))
  (if (not (<= Damage 0.0))
    (bind _output_get (Variables|Default|SetHealth (Math|Float|Clamp(Float) (- (Variables|Default|GetHealth) Damage) 0.0 (Variables|Default|GetMaxHealth))))
    (Default|CallHandleRadialDamage self Damage _output_get DamageType Origin HitInfo InstigatedBy DamageCauser)))